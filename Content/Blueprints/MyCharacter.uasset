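; Player character Blueprint that runs quick-time-event button combat when an enemy attacks.
; IsUnderAttack locks movement, then after a delay faces the enemy, randomizes an A/B/X prompt widget, sets the matching enemy animation and times the response.
; Any press, right or wrong, resets time dilation, clears prompts and costs an enemy life, looping until the enemy dies and is destroyed.
; Player life loss and whistle noise logic are unwired.
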(event `self.ReceiveTick`
  (params (DeltaSeconds :type "Float (single-precision)"))
  ;[1 1 1] Setting The Timer
  (if (`self.IsTiming`)
    (set `self.ElapsedTime` (+ (`self.ElapsedTime`) DeltaSeconds))))

(event `self.ReceiveBeginPlay`
  ;[1 1 1] Create The UIWidgets at beggining of play
  (bind _returnvalue (`|CreateWidget` "/Game/UIWIdgets/UIWidget_A.UIWidget_A_C"))
  (set `self.WidgetA` _returnvalue)
  (bind _returnvalue_2 (`|CreateWidget` "/Game/UIWIdgets/UIWidget_B.UIWidget_B_C"))
  (set `self.Widget B` _returnvalue_2)
  (bind _returnvalue_3 (`|CreateWidget` "/Game/UIWIdgets/UIWidget_X.UIWidget_X_C"))
  (set `self.Widget X` _returnvalue_3)
  (set `self.isInCombat` false))

(event `IsUnderAttack`
  (params (`Who Is Attacking` :type "Actor Object Reference"))
  ;[1 1 1] Entering Fighting State
  (`PlayerController.SetIgnoreMoveInput` (`GameplayStatics.GetPlayerController` null) true)
  (set `self.Enemy Actor` `Who Is Attacking`)
  (bind _asenemycharacter_c (cast `/Game/Animations/EnemyCharacter/Enemy/EnemyCharacter` `Who Is Attacking`))
  (bind _asherotpp_animblueprint_c (cast `/Game/Character/HeroTPP_AnimBlueprint` (`SkeletalMeshComponent.GetAnimInstance` (`Character.Mesh` _asenemycharacter_c))))
  (message `/Game/Animations/EnemyCharacter/Blueprint_For_Behaviour_Tree/BP_AnimInterface.Set_Animation_State` _asherotpp_animblueprint_c 1)
  (`KismetSystemLibrary.Delay` null 0.867 :!label _label)
  (`|ExecutionSequence`
    (:`then_0`
      ;[1 1 1] Player Faces Enemy
      (`self.SetActorRotation` (`KismetMathLibrary.MakeRot` 0.0 (.yaw (`KismetMathLibrary.FindLookAtRotation` (`self.K2_GetActorLocation`) (`self.K2_GetActorLocation` `Who Is Attacking`))))))
    (:`then_2`
      ;[1 1 1] Randomising Buttons
      (set `self.TargetButton` (`KismetMathLibrary.RandomIntegerInRange` (`self.Min`) (`self.Max`))))
    (:`then_3`
      ;[1 1 1] link randomise button to UIWidget
      (`self.ShowCorrectButtonPressWidget`))
    (:`then_4`
      ;[1 1 1] Start Timer
      (set `self.IsTiming` true)
      (set `self.ElapsedTime` 0.0))
    (:`then_5`
      ;[1 1 1] Link randomise button to animation
      (`self.Play Correct Animation`))
    (:`then_6`
      ;[1 1 1] Stop Button From action until in action
      (set `self.isInCombat` true))))

(event `InputAction|Make Noise`
  ;[1 1 1] Making a noise
)

(event `InputAction|A_BUTTON`
  (bind _enemy_actor (`self.Enemy Actor`))
  (bind _returnvalue (`KismetStringLibrary.Conv_DoubleToString` (`self.ElapsedTime`)))
  (bind _returnvalue_2 (`KismetStringLibrary.Conv_IntToString` (`self.Enemy Lives`)))
  ;[1 1 1] Checking If Correct Button is Pressed
  (:`Pressed`
    (if (`self.isInCombat`)
      (if (== (`self.TargetButton`) 2)
        (`self.Success Button Press` :!label _label_2)
        (set `self.IsTiming` false)
        (`KismetSystemLibrary.PrintString` null _returnvalue false)
        (else
          (`self.Fail Button Press` :!label _label_3)
          (set `self.IsTiming` false)
          (`KismetSystemLibrary.PrintString` null (`self.Incorrect Button Press`) false true (struct :`R` 1.0 :`B` 0.401533 :`A` 1.0))
          (`KismetSystemLibrary.PrintString` null _returnvalue false)))
      ;[1 1 1] If pressed correctly, enemy will lose a life
      (set `self.Enemy Lives` (- (`self.Enemy Lives`) (`self.LoseLife`)))
      ;[1 1 1] Check if enemies has 0 lives, if False replay the Sequence
      (if (== (`self.Enemy Lives`) 0)
        ;[1 1 1] If Branch equals true, play death animation and destroy actor from world.
        (`KismetSystemLibrary.PrintString` null _returnvalue_2 true false)
        (`KismetSystemLibrary.PrintString` null "ENEMY HAS DIED!")
        (set `self.isInCombat` false)
        (`PlayerController.SetIgnoreMoveInput` (`GameplayStatics.GetPlayerController` null) false)
        (bind _asenemycharacter_c (cast `/Game/Animations/EnemyCharacter/Enemy/EnemyCharacter` _enemy_actor))
        (bind _asherotpp_animblueprint_c (cast `/Game/Character/HeroTPP_AnimBlueprint` (`SkeletalMeshComponent.GetAnimInstance` (`Character.Mesh` _asenemycharacter_c))))
        (`/Game/Character/HeroTPP_AnimBlueprint.Set_Animation_State` _asherotpp_animblueprint_c 5)
        (`BlackboardComponent.SetValueAsBool` (`AIBlueprintHelperLibrary.GetBlackboard` _asenemycharacter_c) (`self.isDead`) true)
        (set `self.EnemyToKill` _enemy_actor)
        (`KismetSystemLibrary.Delay` null 4.4)
        (`self.K2_DestroyActor` (`self.EnemyToKill`))
        (set `self.Enemy Lives` 3)
        (else
          (`KismetSystemLibrary.PrintString` null _returnvalue_2 true false)
          (goto _label))))))

(event `InputAction|B_BUTTON`
  ;[1 1 1] Checking If Correct Button is Pressed
  (:`Pressed`
    (if (`self.isInCombat`)
      (if (== (`self.TargetButton`) 3)
        (goto _label_2)
        (else
          (goto _label_3))))))

(event `InputAction|X_BUTTON`
  ;[1 1 1] Checking If Correct Button is Pressed
  (:`Pressed`
    (if (`self.isInCombat`)
      (if (== (`self.TargetButton`) 4)
        (goto _label_2)
        (else
          (goto _label_3))))))

(fn `DeathComesToAll`)

(fn `Fail Button Press`
  (`|ExecutionSequence`
    (:`then_0`
      (`GameplayStatics.SetGlobalTimeDilation` null (`self.dilationReset`)))
    (:`then_1`
      (`UserWidget.RemoveFromViewport` (`self.Widget X`))
      (`UserWidget.RemoveFromViewport` (`self.Widget B`))
      (`UserWidget.RemoveFromViewport` (`self.WidgetA`)))))

(fn `Play Correct Animation`
  (bind _asenemycharacter_c (cast `/Game/Animations/EnemyCharacter/Enemy/EnemyCharacter` (`self.Enemy Actor`)))
  (bind _asherotpp_animblueprint_c (cast `/Game/Character/HeroTPP_AnimBlueprint` (`SkeletalMeshComponent.GetAnimInstance` (`Character.Mesh` _asenemycharacter_c))))
  (`/Game/Character/HeroTPP_AnimBlueprint.Set_Animation_State` _asherotpp_animblueprint_c (`self.TargetButton`)))

(fn `ShowCorrectButtonPressWidget`
  (switch `int` (`self.TargetButton`)
    (:`2`
      (`UserWidget.AddToViewport` (`self.WidgetA`)))
    (:`3`
      (`UserWidget.AddToViewport` (`self.Widget B`)))
    (:`4`
      (`UserWidget.AddToViewport` (`self.Widget X`)))))

(fn `Success Button Press`
  (`|ExecutionSequence`
    (:`then_0`
      (`GameplayStatics.SetGlobalTimeDilation` null (`self.dilationReset`)))
    (:`then_1`
      (`UserWidget.RemoveFromViewport` (`self.Widget X`))
      (`UserWidget.RemoveFromViewport` (`self.Widget B`))
      (`UserWidget.RemoveFromViewport` (`self.WidgetA`)))))

(fn `UserConstructionScript`)